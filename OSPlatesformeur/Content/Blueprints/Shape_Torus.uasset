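; Torus shape actor that acts as an elevator, moving its static mesh between a start and an end location.
; EvenementMonter reverses the Elevation timeline at once when EnHaut is set, otherwise plays it after a short delay if the mesh is idle.
; The timeline's Courbe track drives the relative-location lerp, and its completion clears EnMouvement and toggles EnHaut.
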(event Custom|EvenementMonter
  (if (Variables|Default|GetenHaut)
    (bind _courbe (Timeline|Elevation Reverse)
      (:Update
        (Variables|Default|SetenMouvement true)
        (Transformation|SetRelativeLocation (Variables|Default|GetStaticMesh) (Math|Vector|Lerp(Vector) (Variables|Default|GetlocationDepart) (Variables|Default|GetlocationFin) _courbe) false false))
      (:Finished
        (Variables|Default|SetenMouvement false)
        (if (Variables|Default|GetenHaut)
          (Variables|Default|SetenHaut false)
          (else
            (Variables|Default|SetenHaut true)))))
    (elif (not (Variables|Default|GetenMouvement))
      (Utilities|FlowControl|Delay 1.0)
      (Timeline|Elevation Play))))

(event EventBeginPlay)

(event Collision|EventActorBeginOverlap
  (params (OtherActor :type Actor%20Object%20Reference)))

(event EventTick
  (params (DeltaSeconds :type Float%20%28single-precision%29)))

(fn ConstructionScript)